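; Bleach prop that the murderer player can inspect or combine with a carried knife or wine glass.
; Inside its trigger box it shows an in-game note and lets E call the matching bleaching event on that item, gated by DoOnce.
; An interface event toggles it between its saved transform and the player's inspection point.
; Tick drives timeline outline glow from Glowiness cached at BeginPlay, creating a dynamic material instance each frame.
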(event `self.ReceiveTick`
  (params (DeltaSeconds :type "Float (single-precision)"))
  ;[1 0.3185 0] Event tick
  (if (`self.Glowiness`)
    ;[1 0.3185 0] activate Hint_Glow
    (bind _returnvalue (`PrimitiveComponent.CreateDynamicMaterialInstance` (`self.bleach_low`) 0 null))
    (bind (_direction _newtrack_0) (`Timeline|Timeline_0`)
      (:`Update`
        (`MaterialInstanceDynamic.SetScalarParameterValue` _returnvalue "OutlineGlowPower (S)" _newtrack_0)))
    (else
      ;[1 0.3185 0] deactivate Hint_Glow
      (bind _returnvalue_2 (`PrimitiveComponent.CreateDynamicMaterialInstance` (`self.bleach_low`) 0 null))
      (bind (_direction_2 _newtrack_0_2) (`Timeline|Timeline_1`)
        (:`Update`
          (`MaterialInstanceDynamic.SetScalarParameterValue` _returnvalue_2 "OutlineGlowPower (S)" _newtrack_0_2))))))

(event `self.ReceiveBeginPlay`
  ;[0.06848 0.2384 0.807] BeginPlay, get Glowiness variable from MurdererScript
  (bind _asmurderer_script (cast `/Game/Blueprints/Character/MurdererScript` (`GameplayStatics.GetPlayerCharacter` 0))
    (:`then`
      (set `self.Glowiness` (`/Game/Blueprints/Character/MurdererScript.Glowiness` _asmurderer_script)))
    (:`CastFailed`
      (`KismetSystemLibrary.PrintString` "cast to failed"))))

(event `self.Box.OnComponentBeginOverlap`
  (params (OverlappedComponent :type "PrimitiveComponent Object Reference") (OtherActor :type "Actor Object Reference") (OtherComp :type "PrimitiveComponent Object Reference") (OtherBodyIndex :type Integer) (bFromSweep :type Boolean) (SweepResult :type "HitResult Structure (by ref)"))
  ;[0 0 1] Combination only possible in triggerbox
  (`|ExecutionSequence`
    (:`then_0`
      (`self.EnableInput` (`GameplayStatics.GetPlayerController` 0))
      (goto _label :!via `Open`))
    (:`then_1`
      (`self.CreateNotes`))))

(event `Key|E`
  (params (Key :type "Key Structure"))
  ;[0 0 1] Combination only possible in triggerbox
  (:`Pressed`
    ;[1 1 1] when E pressed, decides whether and which event is played
    (`/Engine/EditorBlueprintResources/StandardMacros.Gate` true :!label _label
      (:`Exit`
        (bind _outactors (`GameplayStatics.GetAllActorsOfClass` "/Game/Blueprints/Character/MurdererScript.MurdererScript_C"))
        (switch `string` (`KismetSystemLibrary.GetClassDisplayName` (`GameplayStatics.GetObjectClass` (`/Game/Blueprints/Character/MurdererScript.PickupActor` (`|GetArrayItem` _outactors))))
          (:`Default`
            ;[1 1 1] executes wine/bleach event in WineGlasBP
            (`KismetSystemLibrary.PrintString` "wrong item; not bleachable"))
          (:`Knife_BP_C`
            ;[0.3185 0 1] execute bleaching knife event in KnifeBP
            (bind _outactors_2 (`GameplayStatics.GetAllActorsOfClass` "/Game/Blueprints/Assets/Knife_BP.Knife_BP_C"))
            (`/Engine/EditorBlueprintResources/StandardMacros.DoOnce` false
              (:`Completed`
                (`/Game/Blueprints/Assets/Knife_BP.BleachingKnife` (`|GetArrayItem` _outactors_2))
                (`KismetSystemLibrary.PrintString` "knife/ bleach event" true true (struct :`G` 0.66 :`B` 1.0 :`A` 1.0) 5.0))))
          (:`WineGlas_BP_C`
            (bind _outactors_3 (`GameplayStatics.GetAllActorsOfClass` "/Game/Blueprints/Assets/WineGlas_BP.WineGlas_BP_C"))
            (`/Engine/EditorBlueprintResources/StandardMacros.DoOnce` false
              (:`Completed`
                (`/Game/Blueprints/Assets/WineGlas_BP.BleachingWineGlass` (`|GetArrayItem` _outactors_3))
                (`KismetSystemLibrary.PrintString` "wine/bleach event" true true (struct :`G` 0.66 :`B` 1.0 :`A` 1.0) 5.0)))))))))

(event `self.Box.OnComponentEndOverlap`
  (params (OverlappedComponent :type "PrimitiveComponent Object Reference") (OtherActor :type "Actor Object Reference") (OtherComp :type "PrimitiveComponent Object Reference") (OtherBodyIndex :type Integer))
  ;[0 0 1] Combination only possible in triggerbox
  (`|ExecutionSequence`
    (:`then_0`
      (`self.DisableInput` (`GameplayStatics.GetPlayerController` 0)))
    (:`then_1`
      (`self.DestroyNotes`))))

(event `CreateNotes`
  ;[1 1 1] execute creation for specific igame notifications
  (bind _outactors (`GameplayStatics.GetAllActorsOfClass` "/Game/Blueprints/Character/MurdererScript.MurdererScript_C"))
  (bind _output (`|GetArrayItem` _outactors))
  (set `/Game/Blueprints/Character/MurdererScript.ObjectNoteTags` (`self.bleach_low`) _output)
  (`/Game/Blueprints/Character/MurdererScript.CreateIngameNotification` _output))

(event `DestroyNotes`
  ;[1 1 1] execute creation for specific igame notifications
  (bind _outactors (`GameplayStatics.GetAllActorsOfClass` "/Game/Blueprints/Character/MurdererScript.MurdererScript_C"))
  (`/Game/Blueprints/Character/MurdererScript.DestroyIngameNotification` (`|GetArrayItem` _outactors)))

(event `/Game/Blueprints/Interfaces/IInteractable.IInspectionPosition`
  ;[1 1 1] Interface - IItemPosition
  (if (`self.IsInInspection`)
    ;;[1 1 1] IsInInspection - false
    (`SceneComponent.K2_SetWorldTransform` (`self.bleach_low`) (`self.SavedTransform`) false false)
    (set `self.IsInInspection` false)
    (else
      ;;[1 1 1] IsInInspection - true
      (set `self.SavedTransform` (`SceneComponent.K2_GetComponentToWorld` (`self.bleach_low`)))
      (bind _asmurderer_script (cast `/Game/Blueprints/Character/MurdererScript` (`GameplayStatics.GetPlayerCharacter` 0)))
      (bind _inspectableobjectposition (`/Game/Blueprints/Character/MurdererScript.InspectableObjectPosition` _asmurderer_script))
      (`SceneComponent.K2_SetRelativeTransform` _inspectableobjectposition (`self.InspectionTransform`) false false)
      (`SceneComponent.K2_SetWorldTransform` (`self.bleach_low`) (`SceneComponent.K2_GetComponentToWorld` _inspectableobjectposition) false false)
      (set `self.IsInInspection` true))))

(fn `UserConstructionScript`)