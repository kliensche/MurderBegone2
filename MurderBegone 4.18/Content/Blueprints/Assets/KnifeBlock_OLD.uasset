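; Knife block interactable where the player inserts the held knife, triggering a cutscene sequence.
; Its trigger box toggles input and in-game notes through MurdererScript, and opens a gate that the PickUpInteract input fires.
; If the held object is Knife_BP, it calls KnifeInBlock, drops the object and plays the sequence.
; Tick runs a glow time check and drives outline glow through timelines, creating dynamic material instances every frame.
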(event `self.ReceiveTick`
  (params (DeltaSeconds :type "Float (single-precision)"))
  (bind _knifeblock_knifeblock_low (`self.knifeblock_knifeblock_low`))
  ;[1 0.3176 0] Event Tick - Animation Glow
  (`self.KnifeBlockGlowinessTimeCounter` DeltaSeconds)
  (if (and (== (`self.GlowinessKnifeBlock`) true) (== (`self.IsKnifeBlockInteracted`) false))
    (bind _returnvalue (`PrimitiveComponent.CreateDynamicMaterialInstance` _knifeblock_knifeblock_low 0 null))
    (bind (_direction _newtrack_0) (`Timeline|Timeline_0`)
      (:`Update`
        (`MaterialInstanceDynamic.SetScalarParameterValue` _returnvalue "OutlineGlowPower (S)" _newtrack_0)))
    (else
      (bind _returnvalue_2 (`PrimitiveComponent.CreateDynamicMaterialInstance` _knifeblock_knifeblock_low 0 null))
      (bind (_direction_2 _newtrack_0_2) (`Timeline|Timeline_1`)
        (:`Update`
          (`MaterialInstanceDynamic.SetScalarParameterValue` _returnvalue_2 "OutlineGlowPower (S)" _newtrack_0_2))))))

(event `CreateNotes`
  ;[1 1 1] execute creation for specific igame notifications
  (bind _outactors (`GameplayStatics.GetAllActorsOfClass` "/Game/Blueprints/Character/MurdererScript.MurdererScript_C"))
  (bind _output (`|GetArrayItem` _outactors))
  (set `/Game/Blueprints/Character/MurdererScript.ObjectNoteTags` (`self.knifeblock_knifeblock_low`) _output)
  (`/Game/Blueprints/Character/MurdererScript.CreateIngameNotification` _output))

(event `DestroyNotes`
  ;[1 1 1] execute creation for specific igame notifications
  (bind _outactors (`GameplayStatics.GetAllActorsOfClass` "/Game/Blueprints/Character/MurdererScript.MurdererScript_C"))
  (`/Game/Blueprints/Character/MurdererScript.DestroyIngameNotification` (`|GetArrayItem` _outactors)))

(event `self.Box.OnComponentBeginOverlap`
  (params (OverlappedComponent :type "PrimitiveComponent Object Reference") (OtherActor :type "Actor Object Reference") (OtherComp :type "PrimitiveComponent Object Reference") (OtherBodyIndex :type Integer) (bFromSweep :type Boolean) (SweepResult :type "HitResult Structure (by ref)"))
  ;[0 0 1] Combination only possible in triggerbox
  (`|ExecutionSequence`
    (:`then_0`
      (`self.EnableInput` (`GameplayStatics.GetPlayerController` 0))
      (goto _label :!via `Open`))
    (:`then_1`
      (`self.CreateNotes`))))

(event `InputAction|PickUpInteract`
  (params (Key :type "Key Structure"))
  ;[0 0 1] Combination only possible in triggerbox
  (:`Pressed`
    (bind _outactors (`GameplayStatics.GetAllActorsOfClass` "/Game/Blueprints/Character/MurdererScript.MurdererScript_C"))
    (bind _output (`|GetArrayItem` _outactors))
    (if (`/Game/Blueprints/Character/MurdererScript.NoPickUp` _output)
      ;[0.3185 0 1] when button pressed, execute knife in block event in KnifeBP
      (`/Engine/EditorBlueprintResources/StandardMacros.Gate` true :!label _label
        (:`Exit`
          (bind _outactors_2 (`GameplayStatics.GetAllActorsOfClass` "/Game/Blueprints/Character/MurdererScript.MurdererScript_C"))
          (bind _output_2 (`|GetArrayItem` _outactors_2))
          (switch `string` (`KismetSystemLibrary.GetClassDisplayName` (`GameplayStatics.GetObjectClass` (`/Game/Blueprints/Character/MurdererScript.PickupActor` _output_2)))
            (:`Default`
              (`KismetSystemLibrary.PrintString` "not right object"))
            (:`knife_BP_C`
              (`|ExecutionSequence`
                (:`then_0`
                  (bind _outactors_3 (`GameplayStatics.GetAllActorsOfClass` "/Game/Blueprints/Assets/Knife_BP.Knife_BP_C"))
                  (`/Engine/EditorBlueprintResources/StandardMacros.DoOnce` false
                    (:`Completed`
                      (`/Game/Blueprints/Assets/Knife_BP.KnifeInBlock` (`|GetArrayItem` _outactors_3))
                      (`KismetSystemLibrary.PrintString` "knife in block" true true (struct :`G` 0.66 :`B` 1.0 :`A` 1.0) 5.0))))
                (:`then_1`
                  ;;[1 1 1] Play Sequence only if knife is in hand
                  (`/Game/Blueprints/Character/MurdererScript.DropObject` _output_2)
                  (`self.DisableInput` (`GameplayStatics.GetPlayerController` 0) null)
                  (`MovieSceneSequencePlayer.Play` (`LevelSequenceActor.SequencePlayer` (`self.KnifeBlockSequence`)))
                  (`self.EnableInput` (`GameplayStatics.GetPlayerController` 0))))))))
      (elif (`/Game/Blueprints/Character/MurdererScript.FoundPickUpObject` _output)
        (if (`/Game/Blueprints/Character/MurdererScript.Is_Holding_Object` _output)
          (goto _label)
          (else
            (`KismetSystemLibrary.PrintString` "picking up")))
        (else
          (goto _label))))))

(event `self.Box.OnComponentEndOverlap`
  (params (OverlappedComponent :type "PrimitiveComponent Object Reference") (OtherActor :type "Actor Object Reference") (OtherComp :type "PrimitiveComponent Object Reference") (OtherBodyIndex :type Integer))
  ;[0 0 1] Combination only possible in triggerbox
  (`|ExecutionSequence`
    (:`then_0`
      (`self.DisableInput` (`GameplayStatics.GetPlayerController` 0)))
    (:`then_1`
      (`self.DestroyNotes`))))

(fn `KnifeBlockGlowinessTimeCounter`
  (params (SavedDeltaTime :type "Float (double-precision)"))
  (bind _timeknifeblock (`self.TimeKnifeBlock`))
  (if (< _timeknifeblock (`self.MaxTimeGlowKnifeBlock`))
    (set `self.MaxTimeGlowKnifeBlock` (+ SavedDeltaTime _timeknifeblock))
    (else
      (`/Engine/EditorBlueprintResources/StandardMacros.DoOnce` false
        (:`Completed`
          (set `self.GlowinessKnifeBlock` true))))))

(fn `UserConstructionScript`)