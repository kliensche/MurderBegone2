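; Police radio prop that plays story voice lines and can be picked up for inspection.
; Overlap enables input and opens a gate, so C plays two voice-overs once, delay-separated, and sets RadioSoundPlayed.
; The collision component toggles an in-game notification through MurdererScript.
; Interface events move the mesh to the player's inspection point, toggling physics, and restore its saved transform on exit or reset.
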(event `self.ReceiveActorEndOverlap`
  (params (OtherActor :type "Actor Object Reference"))
  ;[0 0 1] Enables Input when overlap
  (if (not (`PrimitiveComponent.IsOverlappingComponent` (`self.PoliceradioCollision`) null))
    (`self.DisableInput` (`GameplayStatics.GetPlayerController` 0))))

(event `Key|C`
  (params (Key :type "Key Structure"))
  ;[0.3185 0 1] when button pressed: plays VoiceOver, set radio sound bool to played, plays second sound after delay
  (:`Pressed`
    (`/Engine/EditorBlueprintResources/StandardMacros.Gate` true :!label _label
      (:`Exit`
        (`/Engine/EditorBlueprintResources/StandardMacros.DoOnce` false
          (:`Completed`
            (`GameplayStatics.PlaySound2D` "/Game/Audio/VoiceOver/PlaceholderGate2/TimerStepOneVOQuestionable.TimerStepOneVOQuestionable")
            (set `self.RadioSoundPlayed?` true)
            (`KismetSystemLibrary.Delay` 9.0)
            (`GameplayStatics.PlaySound2D` "/Game/Audio/VoiceOver/PlaceholderGate2/ReactionToTimerVO.ReactionToTimerVO")))))))

(event `self.ReceiveActorBeginOverlap`
  (params (OtherActor :type "Actor Object Reference"))
  ;[0 0 1] Enables Input when overlap
  (`KismetSystemLibrary.PrintText` "Police Radio")
  (`self.EnableInput` (`GameplayStatics.GetPlayerController` 0))
  (goto _label :!via `Open`))

(event `self.PoliceradioCollision.OnComponentBeginOverlap`
  (params (OverlappedComponent :type "PrimitiveComponent Object Reference") (OtherActor :type "Actor Object Reference") (OtherComp :type "PrimitiveComponent Object Reference") (OtherBodyIndex :type Integer) (bFromSweep :type Boolean) (SweepResult :type "HitResult Structure (by ref)"))
  ;[1 1 1] execute creation for specific igame notifications
  (bind _outactors (`GameplayStatics.GetAllActorsOfClass` "/Game/Blueprints/Character/MurdererScript.MurdererScript_C"))
  (bind _output (`|GetArrayItem` _outactors))
  (set `/Game/Blueprints/Character/MurdererScript.ObjectNoteTags` (`self.PoliceRadioMesh`) _output)
  (`/Game/Blueprints/Character/MurdererScript.CreateIngameNotification` _output))

(event `self.PoliceradioCollision.OnComponentEndOverlap`
  (params (OverlappedComponent :type "PrimitiveComponent Object Reference") (OtherActor :type "Actor Object Reference") (OtherComp :type "PrimitiveComponent Object Reference") (OtherBodyIndex :type Integer))
  ;[1 1 1] execute creation for specific igame notifications
  (bind _outactors (`GameplayStatics.GetAllActorsOfClass` "/Game/Blueprints/Character/MurdererScript.MurdererScript_C"))
  (`/Game/Blueprints/Character/MurdererScript.DestroyIngameNotification` (`|GetArrayItem` _outactors)))

(event `/Game/Blueprints/Interfaces/IInteractable.IInteract`
  ;[1 1 1] Interface - Interact
  (if (not (`self.isKnifeInteracted`))
    (set `self.isKnifeInteracted` true)))

(event `/Game/Blueprints/Interfaces/IInteractable.IInspectionPosition`
  ;[1 1 1] Interface - IItemPosition
  (if (`self.IsInInspection`)
    ;;[1 1 1] IsInInspection - false
    (`PrimitiveComponent.SetSimulatePhysics` (`self.PoliceRadioMesh`) true)
    (`SceneComponent.K2_SetWorldTransform` (`self.PoliceRadioMesh`) (`self.SavedTransform`) false false)
    (`PrimitiveComponent.SetCollisionResponseToChannel` (`self.PoliceRadioMesh`) "ECC_PhysicsBody" "ECR_Block")
    (set `self.IsInInspection` false)
    (else
      ;;[1 1 1] IsInInspection - true
      (set `self.SavedTransform` (`SceneComponent.K2_GetComponentToWorld` (`self.PoliceRadioMesh`)))
      (bind _asmurderer_script (cast `/Game/Blueprints/Character/MurdererScript` (`GameplayStatics.GetPlayerCharacter` 0)))
      (bind _inspectableobjectposition (`/Game/Blueprints/Character/MurdererScript.InspectableObjectPosition` _asmurderer_script))
      (`SceneComponent.K2_SetRelativeTransform` _inspectableobjectposition (`self.InspectionTransform`) false false)
      (`SceneComponent.K2_SetWorldTransform` (`self.PoliceRadioMesh`) (`SceneComponent.K2_GetComponentToWorld` _inspectableobjectposition) false false)
      (`PrimitiveComponent.SetSimulatePhysics` (`self.PoliceRadioMesh`) false)
      (`PrimitiveComponent.SetCollisionResponseToChannel` (`self.PoliceRadioMesh`) "ECC_PhysicsBody" "ECR_Ignore")
      (set `self.IsInInspection` true))))

(event `/Game/Blueprints/Interfaces/IInteractable.IPositionReset`
  ;[1 1 1] IsInInspection - setFalse if linetrace misses
  (if (`self.IsInInspection`)
    (`PrimitiveComponent.SetSimulatePhysics` (`self.PoliceRadioMesh`) true)
    (`SceneComponent.K2_SetWorldTransform` (`self.PoliceRadioMesh`) (`self.SavedTransform`) false false)
    (set `self.IsInInspection` false)
    (else
      (`KismetSystemLibrary.PrintString` "Dont Reset"))))

(fn `UserConstructionScript`)