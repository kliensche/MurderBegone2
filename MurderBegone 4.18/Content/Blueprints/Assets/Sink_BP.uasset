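; Interactable sink where the player washes a held knife or wine glass.
; UITrigger overlap enables input, opens a gate and shows a note via MurdererScript; PickUpInteract then runs the delay-timed tap animation, water and sound.
; A tagged knife or glass also plays its Level Sequence once, with input disabled; otherwise only the tap runs.
; Separately, Capsule overlap with either item fires its washing event through a DoOnce.
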(event `self.Capsule.OnComponentBeginOverlap`
  (params (OverlappedComponent :type "PrimitiveComponent Object Reference") (OtherActor :type "Actor Object Reference") (OtherComp :type "PrimitiveComponent Object Reference") (OtherBodyIndex :type Integer) (bFromSweep :type Boolean) (SweepResult :type "HitResult Structure (by ref)"))
  ;[0 0 1] on overlap (knife and water) -> executes Washing Events (if possible)
  (switch `string` (`KismetSystemLibrary.GetClassDisplayName` (`GameplayStatics.GetObjectClass` OtherActor))
    (:`Knife_BP_C`
      ;[1 1 1] executes washing knife event in knife bp
      (bind _outactors (`GameplayStatics.GetAllActorsOfClass` "/Game/Blueprints/Assets/Knife_BP.Knife_BP_C"))
      (`/Engine/EditorBlueprintResources/StandardMacros.DoOnce` false
        (:`Completed`
          (`/Game/Blueprints/Assets/Knife_BP.WashingKnife` (`|GetArrayItem` _outactors))
          (`KismetSystemLibrary.PrintString` "wash knife event"))))
    (:`WineGlas_BP_C`
      (`KismetSystemLibrary.PrintString` "animation glass")
      ;[1 1 1] executes washing wine glass event in winglasBP
      (bind _outactors_2 (`GameplayStatics.GetAllActorsOfClass` "/Game/Blueprints/Assets/WineGlas_BP.WineGlas_BP_C"))
      (`/Engine/EditorBlueprintResources/StandardMacros.DoOnce` false
        (:`Completed`
          (`/Game/Blueprints/Assets/WineGlas_BP.WashingWineGlass` (`|GetArrayItem` _outactors_2))
          (`KismetSystemLibrary.PrintString` "wash/wine event"))))))

(event `self.UI Trigger.OnComponentBeginOverlap`
  (params (OverlappedComponent :type "PrimitiveComponent Object Reference") (OtherActor :type "Actor Object Reference") (OtherComp :type "PrimitiveComponent Object Reference") (OtherBodyIndex :type Integer) (bFromSweep :type Boolean) (SweepResult :type "HitResult Structure (by ref)"))
  ;[0.3185 0 1] Overlap_Trigger and Press "E"
  (`|ExecutionSequence`
    (:`then_0`
      (`self.EnableInput` (`GameplayStatics.GetPlayerController` 0))
      (goto _label :!via `Open`))
    (:`then_1`
      (`self.CreateNotes`))))

(event `InputAction|PickUpInteract`
  (params (Key :type "Key Structure"))
  ;[0.3185 0 1] Overlap_Trigger and Press "E"
  (:`Pressed`
    (bind _outactors (`GameplayStatics.GetAllActorsOfClass` "/Game/Blueprints/Character/MurdererScript.MurdererScript_C"))
    (bind _output (`|GetArrayItem` _outactors))
    (if (`/Game/Blueprints/Character/MurdererScript.NoPickUp` _output)
      ;[1 1 1] logic, whether and what object interact with sink and play right animation
      (`/Engine/EditorBlueprintResources/StandardMacros.Gate` true :!label _label
        (:`Exit`
          (if (`/Game/Blueprints/Character/MurdererScript.Is_Holding_Object` _output)
            (bind _pickupactor (`/Game/Blueprints/Character/MurdererScript.PickupActor` _output))
            (if (`self.ActorHasTag` _pickupactor "knife")
              (if (`self.IsSquencePlayedKnife`)
                (`KismetSystemLibrary.PrintString` "sequence already played" :!label _label_2)
                ;[1 0 0] Tap_Animation_and_Sequence
                ;;[1 1 1] only opens sink and water + sound
                (`self.DisableInput` (`GameplayStatics.GetPlayerController` 0) null :!label _label_3)
                (`AudioComponent.Play` (`self.Tab`) 0.0)
                (`SkeletalMeshComponent.PlayAnimation` (`self.Sink_new`) "/Game/VFX/Sink/Anim/Sink_new_TabClose_Anim.Sink_new_TabClose_Anim" false)
                (`KismetSystemLibrary.Delay` 3.3333) ; delay to wait for Tab_Anim
                (`SceneComponent.ToggleVisibility` (`self.Sink_water`) false)
                (set `self.IsTapOpen` true)
                (`AudioComponent.Play` (`self.Water_Start`) 0.0)
                (`KismetSystemLibrary.Delay` 5.0) ; Time for Waterflow
                (`AudioComponent.Play` (`self.Tab`) 0.0)
                (`SkeletalMeshComponent.PlayAnimation` (`self.Sink_new`) "/Game/VFX/Sink/Anim/Sink_new_TabClose_Anim.Sink_new_TabClose_Anim" false)
                (`AudioComponent.Play` (`self.Water_End`) 0.0)
                (`KismetSystemLibrary.Delay` 3.3333)
                (`SceneComponent.ToggleVisibility` (`self.Sink_water`) false)
                (`AudioComponent.Stop` (`self.Water_Start`))
                (`self.EnableInput` (`GameplayStatics.GetPlayerController` 0))
                (else
                  ;;[1 1 1] Play Sequence only if knife is in hand
                  (`self.SetActorHiddenInGame` _pickupactor false)
                  (`self.DisableInput` (`GameplayStatics.GetPlayerController` 0) null)
                  (`MovieSceneSequencePlayer.Play` (`LevelSequenceActor.SequencePlayer` (`self.Sink_Sequence_Knife`)))
                  (`AudioComponent.Play` (`self.Tab`) 0.0)
                  (`SkeletalMeshComponent.PlayAnimation` (`self.Sink_new`) "/Game/VFX/Sink/Anim/Sink_new_TabClose_Anim.Sink_new_TabClose_Anim" false)
                  (`KismetSystemLibrary.Delay` 3.3333) ; delay to wait for Tab_Anim
                  (`SceneComponent.ToggleVisibility` (`self.Sink_water`) false)
                  (set `self.IsTapOpen` true)
                  (`AudioComponent.Play` (`self.Water_Start`) 0.0)
                  (`KismetSystemLibrary.Delay` 5.0) ; Time for Waterflow
                  (`AudioComponent.Play` (`self.Tab`) 0.0)
                  (`SkeletalMeshComponent.PlayAnimation` (`self.Sink_new`) "/Game/VFX/Sink/Anim/Sink_new_TabClose_Anim.Sink_new_TabClose_Anim" false)
                  (`AudioComponent.Play` (`self.Water_End`) 0.0)
                  (`KismetSystemLibrary.Delay` 3.3333)
                  (`SceneComponent.ToggleVisibility` (`self.Sink_water`) false)
                  (`AudioComponent.Stop` (`self.Water_Start`))
                  (set `self.IsSquencePlayedKnife` true)
                  (`self.SetActorHiddenInGame` _pickupactor true)
                  (`self.EnableInput` (`GameplayStatics.GetPlayerController` 0))))
              (elif (`self.ActorHasTag` _pickupactor "glass")
                (if (`self.IsSquencePlayedGlass`)
                  (goto _label_2)
                  (else
                    ;;[1 1 1] Play Sequence only if glass is in hand
                    (`self.SetActorHiddenInGame` _pickupactor false)
                    (`self.DisableInput` (`GameplayStatics.GetPlayerController` 0) null)
                    (`MovieSceneSequencePlayer.Play` (`LevelSequenceActor.SequencePlayer` (`self.Sink_Sequence_Glass_0`)))
                    (`AudioComponent.Play` (`self.Tab`) 0.0)
                    (`SkeletalMeshComponent.PlayAnimation` (`self.Sink_new`) "/Game/VFX/Sink/Anim/Sink_new_TabClose_Anim.Sink_new_TabClose_Anim" false)
                    (`KismetSystemLibrary.Delay` 3.3333) ; delay to wait for Tab_Anim
                    (`SceneComponent.ToggleVisibility` (`self.Sink_water`) false)
                    (set `self.IsTapOpen` true)
                    (`AudioComponent.Play` (`self.Water_Start`) 0.0)
                    (`KismetSystemLibrary.Delay` 5.0) ; Time for Waterflow
                    (`AudioComponent.Play` (`self.Tab`) 0.0)
                    (`SkeletalMeshComponent.PlayAnimation` (`self.Sink_new`) "/Game/VFX/Sink/Anim/Sink_new_TabClose_Anim.Sink_new_TabClose_Anim" false)
                    (`AudioComponent.Play` (`self.Water_End`) 0.0)
                    (`KismetSystemLibrary.Delay` 3.3333)
                    (`SceneComponent.ToggleVisibility` (`self.Sink_water`) false)
                    (`AudioComponent.Stop` (`self.Water_Start`))
                    (set `self.IsSquencePlayedGlass` true)
                    (`self.SetActorHiddenInGame` _pickupactor true)
                    (`self.EnableInput` (`GameplayStatics.GetPlayerController` 0))))
                (else
                  (`KismetSystemLibrary.PrintString` "not right object")
                  (goto _label_3))))
            (else
              (`KismetSystemLibrary.PrintString` "not holding anything")
              (goto _label_3)))))
      (elif (`/Game/Blueprints/Character/MurdererScript.FoundPickUpObject` _output)
        (if (`/Game/Blueprints/Character/MurdererScript.Is_Holding_Object` _output)
          (goto _label)
          (else
            (`KismetSystemLibrary.PrintString` "picking up")))
        (else
          (goto _label))))))

(event `self.UI Trigger.OnComponentEndOverlap`
  (params (OverlappedComponent :type "PrimitiveComponent Object Reference") (OtherActor :type "Actor Object Reference") (OtherComp :type "PrimitiveComponent Object Reference") (OtherBodyIndex :type Integer))
  ;[0.3185 0 1] Overlap_Trigger and Press "E"
  (`|ExecutionSequence`
    (:`then_0`
      (`self.DisableInput` (`GameplayStatics.GetPlayerController` 0)))
    (:`then_1`
      (`self.DestroyNotes`))))

(event `CreateNotes`
  ;[1 1 1] execute creation for specific igame notifications
  (bind _outactors (`GameplayStatics.GetAllActorsOfClass` "/Game/Blueprints/Character/MurdererScript.MurdererScript_C"))
  (bind _output (`|GetArrayItem` _outactors))
  (set `/Game/Blueprints/Character/MurdererScript.ObjectNoteTags` (`self.Sink_new`) _output)
  (`/Game/Blueprints/Character/MurdererScript.CreateIngameNotification` _output))

(event `DestroyNotes`
  ;[1 1 1] execute creation for specific igame notifications
  (bind _outactors (`GameplayStatics.GetAllActorsOfClass` "/Game/Blueprints/Character/MurdererScript.MurdererScript_C"))
  (`/Game/Blueprints/Character/MurdererScript.DestroyIngameNotification` (`|GetArrayItem` _outactors)))

(fn `UserConstructionScript`)