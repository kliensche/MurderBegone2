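; Exit door actor that lets the player press E nearby to bring up an exit confirmation.
; Beginning an overlap prints a prompt, enables input and opens a gate; ending it disables input once DoorCollision is clear.
; E passes the gate to show the ConfirmExit widget with cursor and UI-only input, calling SetGamePaused with false despite its pause comment.
; The first use also plays the DoorIncompleteVO voice-over through a DoOnce.
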(event `self.ReceiveActorEndOverlap`
  (params (OtherActor :type "Actor Object Reference"))
  ;[0 0 1] enable input when overlap
  (if (not (`PrimitiveComponent.IsOverlappingComponent` (`self.DoorCollision`) null))
    (`self.DisableInput` (`GameplayStatics.GetPlayerController` 0))))

(event `Key|E`
  (params (Key :type "Key Structure"))
  (bind _returnvalue (`GameplayStatics.GetPlayerController` 0))
  ;[0 0 1] enable input when overlap
  (:`Pressed`
    (`/Engine/EditorBlueprintResources/StandardMacros.Gate` true :!label _label
      (:`Exit`
        (`|ExecutionSequence`
          (:`then_0`
            ;[0.3185 0 1] Create ConfirmExitWidget, gets mouse cursor, pauses game
            (bind _returnvalue_2 (`|CreateWidget` "/Game/Blueprints/UI/ConfirmExit.ConfirmExit_C"))
            (`UserWidget.AddToViewport` _returnvalue_2 0)
            (set `PlayerController.bShowMouseCursor` true _returnvalue)
            (`GameplayStatics.SetGamePaused` false)
            (`WidgetBlueprintLibrary.SetInputMode_UIOnlyEx` _returnvalue))
          (:`then_1`
            ;[0.3185 0 1] plays VoiceOver
            (`/Engine/EditorBlueprintResources/StandardMacros.DoOnce` false
              (:`Completed`
                (`GameplayStatics.PlaySound2D` "/Game/Audio/VoiceOver/PlaceholderGate2/DoorIncompleteVO.DoorIncompleteVO")))))))))

(event `self.ReceiveActorBeginOverlap`
  (params (OtherActor :type "Actor Object Reference"))
  ;[0 0 1] enable input when overlap
  (`KismetSystemLibrary.PrintText` "Exit ?")
  (`self.EnableInput` (`GameplayStatics.GetPlayerController` 0))
  (goto _label :!via `Open`))

(fn `UserConstructionScript`)