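; Knife block prop that glows as a hint and shows an in-game note through MurdererScript while something overlaps its trigger.
; Tick runs a time check for the glow flag, recreates a dynamic material and plays one of two timelines driving outline glow power.
; The trigger also toggles input, but interacting only prints a debug message.
; Gated knife-placement logic with its sequence playback is present but never runs.
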(event `self.ReceiveTick`
  (params (DeltaSeconds :type "Float (single-precision)"))
  (bind _knifeblock_knifeblock_low (`self.knifeblock_knifeblock_low`))
  ;[1 0.3176 0] Event Tick - Animation Glow
  (`self.KnifeBlockGlowinessTimeCounter` DeltaSeconds)
  (if (and (== (`self.GlowinessKnifeBlock`) true) (== (`self.IsKnifeBlockInteracted`) false))
    (bind _returnvalue (`PrimitiveComponent.CreateDynamicMaterialInstance` _knifeblock_knifeblock_low 0 null))
    (bind (_direction _newtrack_0) (`Timeline|Timeline_0`)
      (:`Update`
        (`MaterialInstanceDynamic.SetScalarParameterValue` _returnvalue "OutlineGlowPower (S)" _newtrack_0)))
    (else
      (bind _returnvalue_2 (`PrimitiveComponent.CreateDynamicMaterialInstance` _knifeblock_knifeblock_low 0 null))
      (bind (_direction_2 _newtrack_0_2) (`Timeline|Timeline_1`)
        (:`Update`
          (`MaterialInstanceDynamic.SetScalarParameterValue` _returnvalue_2 "OutlineGlowPower (S)" _newtrack_0_2))))))

(event `CreateNotes`
  ;[1 1 1] execute creation for specific igame notifications
  (bind _outactors (`GameplayStatics.GetAllActorsOfClass` "/Game/Blueprints/Character/MurdererScript.MurdererScript_C"))
  (bind _output (`|GetArrayItem` _outactors))
  (set `/Game/Blueprints/Character/MurdererScript.ObjectNoteTags` (`self.knifeblock_knifeblock_low`) _output)
  (`/Game/Blueprints/Character/MurdererScript.CreateIngameNotification` _output))

(event `DestroyNotes`
  ;[1 1 1] execute creation for specific igame notifications
  (bind _outactors (`GameplayStatics.GetAllActorsOfClass` "/Game/Blueprints/Character/MurdererScript.MurdererScript_C"))
  (`/Game/Blueprints/Character/MurdererScript.DestroyIngameNotification` (`|GetArrayItem` _outactors)))

(event `self.UI Trigger.OnComponentBeginOverlap`
  (params (OverlappedComponent :type "PrimitiveComponent Object Reference") (OtherActor :type "Actor Object Reference") (OtherComp :type "PrimitiveComponent Object Reference") (OtherBodyIndex :type Integer) (bFromSweep :type Boolean) (SweepResult :type "HitResult Structure (by ref)"))
  ;[0.3185 0 1] Overlap_Trigger and Press "E"
  (`|ExecutionSequence`
    (:`then_0`
      (`self.EnableInput` (`GameplayStatics.GetPlayerController` 0)))
    (:`then_1`
      (`self.CreateNotes`))))

(event `InputAction|PickUpInteract`
  (params (Key :type "Key Structure"))
  ;[0.3185 0 1] Overlap_Trigger and Press "E"
  (:`Pressed`
    (bind _outactors (`GameplayStatics.GetAllActorsOfClass` "/Game/Blueprints/Character/MurdererScript.MurdererScript_C"))
    (bind _output (`|GetArrayItem` _outactors))
    (if (`/Game/Blueprints/Character/MurdererScript.NoPickUp` _output)
      _
      (elif (`/Game/Blueprints/Character/MurdererScript.FoundPickUpObject` _output)
        (if (not (`/Game/Blueprints/Character/MurdererScript.Is_Holding_Object` _output))
          (`KismetSystemLibrary.PrintString` "picking up"))))))

(event `self.UI Trigger.OnComponentEndOverlap`
  (params (OverlappedComponent :type "PrimitiveComponent Object Reference") (OtherActor :type "Actor Object Reference") (OtherComp :type "PrimitiveComponent Object Reference") (OtherBodyIndex :type Integer))
  ;[0.3185 0 1] Overlap_Trigger and Press "E"
  (`|ExecutionSequence`
    (:`then_0`
      (`self.DisableInput` (`GameplayStatics.GetPlayerController` 0)))
    (:`then_1`
      (`self.DestroyNotes`))))

(fn `KnifeBlockGlowinessTimeCounter`
  (params (SavedDeltaTime :type "Float (double-precision)"))
  (bind _timeknifeblock (`self.TimeKnifeBlock`))
  (if (< _timeknifeblock (`self.MaxTimeGlowKnifeBlock`))
    (set `self.MaxTimeGlowKnifeBlock` (+ SavedDeltaTime _timeknifeblock))
    (else
      (`/Engine/EditorBlueprintResources/StandardMacros.DoOnce` false
        (:`Completed`
          (set `self.GlowinessKnifeBlock` true))))))

(fn `UserConstructionScript`)