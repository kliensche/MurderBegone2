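; NewCaseFilesBP is a case files prop the player can interact with and pick up for inspection.
; Interacting sets a one-time flag.
; Inspection toggles: it saves the mesh transform, snaps it to MurdererScript's InspectableObjectPosition offset by InspectionTransform, and disables physics and PhysicsBody blocking, then restores all three.
; A separate reset event, noted for linetrace misses, restores transform and physics but leaves collision ignored.
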(event `/Game/Blueprints/Interfaces/IInteractable.IInteract`
  ;[1 1 1] Interface - Interact
  (if (not (`self.IsCaseFilesInteracted`))
    (set `self.IsCaseFilesInteracted` true)))

(event `/Game/Blueprints/Interfaces/IInteractable.IInspectionPosition`
  (bind _staticmeshcomponent (`self.StaticMeshComponent`))
  ;[1 1 1] Interface - IItemPosition
  (if (`self.IsInInspection`)
    ;;[1 1 1] IsInInspection - false
    (`PrimitiveComponent.SetSimulatePhysics` (`self.StaticMeshComponent`) true)
    (`SceneComponent.K2_SetWorldTransform` (`self.StaticMeshComponent`) (`self.SavedTransform`) false false)
    (`PrimitiveComponent.SetCollisionResponseToChannel` (`self.StaticMeshComponent`) "ECC_PhysicsBody" "ECR_Block")
    (set `self.IsInInspection` false)
    (else
      ;;[1 1 1] IsInInspection - true
      (set `self.SavedTransform` (`SceneComponent.K2_GetComponentToWorld` (`self.StaticMeshComponent`)))
      (bind _asmurderer_script (cast `/Game/Blueprints/Character/MurdererScript` (`GameplayStatics.GetPlayerCharacter` 0)))
      (bind _inspectableobjectposition (`/Game/Blueprints/Character/MurdererScript.InspectableObjectPosition` _asmurderer_script))
      (`SceneComponent.K2_SetRelativeTransform` _inspectableobjectposition (`self.InspectionTransform`) false false)
      (`SceneComponent.K2_SetWorldTransform` (`self.StaticMeshComponent`) (`SceneComponent.K2_GetComponentToWorld` _inspectableobjectposition) false false)
      (`PrimitiveComponent.SetSimulatePhysics` _staticmeshcomponent false)
      (`PrimitiveComponent.SetCollisionResponseToChannel` _staticmeshcomponent "ECC_PhysicsBody" "ECR_Ignore")
      (set `self.IsInInspection` true))))

(event `/Game/Blueprints/Interfaces/IInteractable.IPositionReset`
  ;[1 1 1] IsInInspection - setFalse if linetrace misses
  (if (`self.IsInInspection`)
    (`PrimitiveComponent.SetSimulatePhysics` (`self.StaticMeshComponent`) true)
    (`SceneComponent.K2_SetWorldTransform` (`self.StaticMeshComponent`) (`self.SavedTransform`) false false)
    (set `self.IsInInspection` false)
    (else
      (`KismetSystemLibrary.PrintString` "Dont Reset"))))

(fn `UserConstructionScript`)