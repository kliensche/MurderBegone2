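; Knife evidence prop that the player can inspect, wash, bleach or return to a knife block.
; Each action raises MurdererScript's event counter for evaluation and updates slot or state values, with washing animated through a dynamic material parameter.
; Interface calls toggle hint glow, applied on Tick via timelines, and move the knife to and from an inspection position using a saved transform.
; UITrigger overlaps toggle the player's notification flag.
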(event `BleachingKnife`
  ;[0.3185 0 1] Bleaching Knife Event: execute raise counter function
  (`GameplayStatics.PlaySound2D` "/Game/Audio/VoiceOver/PlaceholderGate2/KnifeBleachVO.KnifeBleachVO")
  (bind (_eventcount _knifebool _asmurdererscript) (`self.RaiseEventCounter`))
  (set `/Game/Blueprints/Character/MurdererScript.isKnifeBleached` _knifebool _asmurdererscript)
  (`KismetSystemLibrary.PrintString` (`KismetStringLibrary.Conv_IntToString` _eventcount))
  (bind _outactors (`GameplayStatics.GetAllActorsOfClass` "/Game/Blueprints/Character/MurdererScript.MurdererScript_C"))
  (bind _output (`|GetArrayItem` _outactors))
  (set `/Game/Blueprints/Character/MurdererScript.SlotItem` 3 _output)
  (set `/Game/Blueprints/Character/MurdererScript.isKnifeBleached` true _output))

(event `WashingKnife`
  (bind _knife (`self.Knife`))
  ;[0.3185 0 1] Washing Knife Event: plays Anim and execute raises counter function
  (`PrimitiveComponent.SetSimulatePhysics` (`self.Knife`) false)
  (bind _returnvalue (`PrimitiveComponent.CreateDynamicMaterialInstance` (`self.Knife`) 0 null))
  (bind (_direction _newtrack_0) (`Timeline|Transition_Anim`)
    (:`Update`
      (`MaterialInstanceDynamic.SetScalarParameterValue` _returnvalue "Time_In (S)" _newtrack_0))
    (:`Finished`
      (bind (_eventcount _knifebool _asmurdererscript) (`self.RaiseEventCounter`))
      (set `/Game/Blueprints/Character/MurdererScript.isKnifeWashed` _knifebool _asmurdererscript)
      (`KismetSystemLibrary.PrintString` (`KismetStringLibrary.Conv_IntToString` _eventcount))
      (bind _outactors (`GameplayStatics.GetAllActorsOfClass` "/Game/Blueprints/Character/MurdererScript.MurdererScript_C"))
      (bind _output (`|GetArrayItem` _outactors))
      (set `/Game/Blueprints/Character/MurdererScript.SlotItem` 2 _output)
      (set `/Game/Blueprints/Character/MurdererScript.isKnifeWashed` true _output)
      (`/Game/Blueprints/Character/MurdererScript.SlotItemIntToWidget` _output)
      (`KismetSystemLibrary.Delay` 2.0)
      (`PrimitiveComponent.SetSimulatePhysics` _knife true)
      (`PrimitiveComponent.SetCollisionResponseToChannel` _knife "ECC_PhysicsBody" "ECR_Block")
      (`/Game/Blueprints/Character/MurdererScript.VOKnifeWash` _output))))

(event `KnifeInBlock`
  ;[0.3185 0 1] Knife Block Event: execute raise counter function
  (`PrimitiveComponent.SetSimulatePhysics` (`self.Knife`) false)
  (bind _eventcount (`self.RaiseEventCounter`))
  (`KismetSystemLibrary.PrintString` "EventCounter Box" true true (struct :`R` 1.0 :`G` 0.015653 :`A` 1.0))
  (`KismetSystemLibrary.PrintString` (`KismetStringLibrary.Conv_IntToString` _eventcount))
  ;[0.3185 0 1] destroys slot item (knife) after putting it in knife block, changes slot images to empty
  (bind _asmurderer_script (cast `/Game/Blueprints/Character/MurdererScript` (`GameplayStatics.GetPlayerCharacter` 0))
    (:`then`
      (if (!= (`/Game/Blueprints/Character/MurdererScript.SlotItem` _asmurderer_script) 0)
        (set `/Game/Blueprints/Character/MurdererScript.SlotItem` 0 _asmurderer_script)
        (`/Game/Blueprints/Character/MurdererScript.SlotItemIntToWidget` _asmurderer_script)
        (set `self.IsKnifeInBlock` true)
        (`/Game/Blueprints/Character/MurdererScript.VOKnifeInBlock` _asmurderer_script)
        (else
          (`KismetSystemLibrary.PrintString` "Failed to set slot item"))))
    (:`CastFailed`
      (`KismetSystemLibrary.PrintString` "cast to failed"))))

(event `self.UI Trigger.OnComponentBeginOverlap`
  (params (OverlappedComponent :type "PrimitiveComponent Object Reference") (OtherActor :type "Actor Object Reference") (OtherComp :type "PrimitiveComponent Object Reference") (OtherBodyIndex :type Integer) (bFromSweep :type Boolean) (SweepResult :type "HitResult Structure (by ref)"))
  ;[1 1 1] execute creation for specific igame notifications
  (bind _asmurderer_script (cast `/Game/Blueprints/Character/MurdererScript` OtherActor)
    (:`then`
      (if (not (or (`/Game/Blueprints/Character/MurdererScript.Is_Holding_Object` _asmurderer_script) (`/Game/Blueprints/Character/MurdererScript.AmIHolding` _asmurderer_script) (`/Game/Blueprints/Character/MurdererScript.NotificationTrigger` _asmurderer_script)))
        (set `/Game/Blueprints/Character/MurdererScript.NotificationTrigger` true _asmurderer_script)))
    (:`CastFailed`
      (`KismetSystemLibrary.PrintString` "Cast failed" true true (struct :`R` 1.0 :`G` 0.938239 :`B` 0.130349 :`A` 1.0)))))

(event `self.ReceiveTick`
  (params (DeltaSeconds :type "Float (single-precision)"))
  ;[1 0.3176 0] Event tick
  (if (`self.GlowinessKnife`)
    ;[1 0.3185 0] activate Hint_Glow
    (bind _returnvalue (`PrimitiveComponent.CreateDynamicMaterialInstance` (`self.Knife`) 0 null))
    (bind (_direction _newtrack_0) (`Timeline|Timeline_0`)
      (:`Update`
        (`MaterialInstanceDynamic.SetScalarParameterValue` _returnvalue "OutlineGlowPower (S)" _newtrack_0)))
    (else
      ;[1 0.3185 0] deactivate Hint_Glow
      (bind _returnvalue_2 (`PrimitiveComponent.CreateDynamicMaterialInstance` (`self.Knife`) 0 null))
      (bind (_direction_2 _newtrack_0_2) (`Timeline|Timeline_1`)
        (:`Update`
          (`MaterialInstanceDynamic.SetScalarParameterValue` _returnvalue_2 "OutlineGlowPower (S)" _newtrack_0_2))))))

(event `self.UI Trigger.OnComponentEndOverlap`
  (params (OverlappedComponent :type "PrimitiveComponent Object Reference") (OtherActor :type "Actor Object Reference") (OtherComp :type "PrimitiveComponent Object Reference") (OtherBodyIndex :type Integer))
  ;[1 1 1] execute creation for specific igame notifications
  (bind _asmurderer_script (cast `/Game/Blueprints/Character/MurdererScript` OtherActor)
    (:`then`
      (if (`/Game/Blueprints/Character/MurdererScript.NotificationTrigger` _asmurderer_script)
        (set `/Game/Blueprints/Character/MurdererScript.NotificationTrigger` false _asmurderer_script)))
    (:`CastFailed`
      (`KismetSystemLibrary.PrintString` "Cast failed" true true (struct :`R` 0.135668 :`G` 1.0 :`B` 0.288385 :`A` 1.0)))))

(event `/Game/Blueprints/Interfaces/IInteractable.IGlow`
  (params (GlowActive :type Boolean))
  ;[1 1 1] Interface - Interact
  (set `self.GlowinessKnife` GlowActive))

(event `/Game/Blueprints/Interfaces/IInteractable.IInteract`)

(event `/Game/Blueprints/Interfaces/IInteractable.IInspectionPosition`
  (bind _knife (`self.Knife`))
  ;[1 1 1] Interface - IItemPosition
  (if (`self.IsInInspection`)
    ;;[1 1 1] IsInInspection - false
    (`PrimitiveComponent.SetSimulatePhysics` (`self.Knife`) true)
    (`SceneComponent.K2_SetWorldTransform` (`self.Knife`) (`self.SavedTransform`) false false)
    (`PrimitiveComponent.SetCollisionResponseToChannel` (`self.Knife`) "ECC_PhysicsBody" "ECR_Block")
    (set `self.IsInInspection` false)
    (else
      ;;[1 1 1] IsInInspection - true
      (set `self.SavedTransform` (`SceneComponent.K2_GetComponentToWorld` (`self.Knife`)))
      (bind _asmurderer_script (cast `/Game/Blueprints/Character/MurdererScript` (`GameplayStatics.GetPlayerCharacter` 0)))
      (bind _inspectableobjectposition (`/Game/Blueprints/Character/MurdererScript.InspectableObjectPosition` _asmurderer_script))
      (`SceneComponent.K2_SetRelativeTransform` _inspectableobjectposition (`self.InspectionTransform`) false false)
      (`SceneComponent.K2_SetWorldTransform` (`self.Knife`) (`SceneComponent.K2_GetComponentToWorld` _inspectableobjectposition) false false)
      (`PrimitiveComponent.SetSimulatePhysics` _knife false)
      (`PrimitiveComponent.SetCollisionResponseToChannel` _knife "ECC_PhysicsBody" "ECR_Ignore")
      (set `self.IsInInspection` true))))

(event `/Game/Blueprints/Interfaces/IInteractable.IPositionReset`
  ;[1 1 1] IsInInspection - setFalse if linetrace misses
  (if (`self.IsInInspection`)
    (`PrimitiveComponent.SetSimulatePhysics` (`self.Knife`) true)
    (`SceneComponent.K2_SetWorldTransform` (`self.Knife`) (`self.SavedTransform`) false false)
    (set `self.IsInInspection` false)
    (else
      (`KismetSystemLibrary.PrintString` "Dont Reset"))))

(fn `KnifeGlowinessTimeCounter`
  (params (SavedDeltaSeconds :type "Float (double-precision)")))

(fn `RaiseEventCounter`
  (returns (EventCount :type Integer) (KnifeBool :type Boolean) (AsMurdererScript :type "/Game/Blueprints/Character/MurdererScript Object Reference"))
  ;[0.3185 0 1] Raises counter for evaluation
  (bind _asmurderer_script (cast `/Game/Blueprints/Character/MurdererScript` (`GameplayStatics.GetPlayerCharacter` 0))
    (:`then`
      (bind _output_get (set `/Game/Blueprints/Character/MurdererScript.eventCounter` (+ (`/Game/Blueprints/Character/MurdererScript.eventCounter` _asmurderer_script) 1) _asmurderer_script))
      (return _output_get true _asmurderer_script))
    (:`CastFailed`
      (`KismetSystemLibrary.PrintString` "cast to failed"))))

(fn `UserConstructionScript`)