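; Photo album actor that the player can inspect, with an outline glow to highlight it.
; Tick creates a dynamic material each frame and plays one of two timelines driving glow power, chosen by a flag the glow interface sets.
; A trigger overlap toggles the player's notification flag.
; Inspection interfaces save the transform, move the mesh to the player's inspection point with physics off, then restore it on toggle or reset.
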(event `self.ReceiveTick`
  (params (DeltaSeconds :type "Float (single-precision)"))
  ;[1 0.3176 0] Event Tick - Animation Glow
  (if (`self.GlowinessPhotoAlbum`)
    (bind _returnvalue (`PrimitiveComponent.CreateDynamicMaterialInstance` (`self.picturealbum_low`) 0 null))
    (bind (_direction _newtrack_0) (`Timeline|Timeline_0`)
      (:`Update`
        (`MaterialInstanceDynamic.SetScalarParameterValue` _returnvalue "OutlineGlowPower (S)" _newtrack_0)))
    (else
      (bind _returnvalue_2 (`PrimitiveComponent.CreateDynamicMaterialInstance` (`self.picturealbum_low`) 0 null))
      (bind (_direction_2 _newtrack_0_2) (`Timeline|Timeline_1`)
        (:`Update`
          (`MaterialInstanceDynamic.SetScalarParameterValue` _returnvalue_2 "OutlineGlowPower (S)" _newtrack_0_2))))))

(event `/Game/Blueprints/Interfaces/IInteractable.IInteract`
  ;[1 1 1] Interface - Interact
  (if (not (`self.IsPhotoAlbumInteracted`))
    (set `self.IsPhotoAlbumInteracted` true)))

(event `self.FotoAlbumTrigger.OnComponentBeginOverlap`
  (params (OverlappedComponent :type "PrimitiveComponent Object Reference") (OtherActor :type "Actor Object Reference") (OtherComp :type "PrimitiveComponent Object Reference") (OtherBodyIndex :type Integer) (bFromSweep :type Boolean) (SweepResult :type "HitResult Structure (by ref)"))
  ;[1 1 1] execute creation for specific igame notifications
  (bind _asmurderer_script (cast `/Game/Blueprints/Character/MurdererScript` OtherActor)
    (:`then`
      (if (not (or (`/Game/Blueprints/Character/MurdererScript.Is_Holding_Object` _asmurderer_script) (`/Game/Blueprints/Character/MurdererScript.AmIHolding` _asmurderer_script) (`/Game/Blueprints/Character/MurdererScript.NotificationTrigger` _asmurderer_script)))
        (set `/Game/Blueprints/Character/MurdererScript.NotificationTrigger` true _asmurderer_script)))
    (:`CastFailed`
      (`KismetSystemLibrary.PrintString` "Overlapped with other object" true true (struct :`R` 1.0 :`G` 0.938239 :`B` 0.130349 :`A` 1.0)))))

(event `self.FotoAlbumTrigger.OnComponentEndOverlap`
  (params (OverlappedComponent :type "PrimitiveComponent Object Reference") (OtherActor :type "Actor Object Reference") (OtherComp :type "PrimitiveComponent Object Reference") (OtherBodyIndex :type Integer))
  ;[1 1 1] execute creation for specific igame notifications
  (bind _asmurderer_script (cast `/Game/Blueprints/Character/MurdererScript` OtherActor))
  (if (`/Game/Blueprints/Character/MurdererScript.NotificationTrigger` _asmurderer_script)
    (set `/Game/Blueprints/Character/MurdererScript.NotificationTrigger` false _asmurderer_script)))

(event `/Game/Blueprints/Interfaces/IInteractable.IGlow`
  (params (GlowActive :type Boolean))
  ;[1 1 1] Interface-Interact
  (set `self.GlowinessPhotoAlbum` GlowActive))

(event `/Game/Blueprints/Interfaces/IInteractable.IInspectionPosition`
  ;[1 1 1] Interface - IItemPosition
  (if (`self.IsInInspection`)
    ;;[1 1 1] IsInInspection - false
    (`PrimitiveComponent.SetSimulatePhysics` (`self.picturealbum_low`) true)
    (`SceneComponent.K2_SetWorldTransform` (`self.picturealbum_low`) (`self.SavedTransform`) false false)
    (`PrimitiveComponent.SetCollisionResponseToChannel` (`self.picturealbum_low`) "ECC_PhysicsBody" "ECR_Block")
    (set `self.IsInInspection` false)
    (else
      ;;[1 1 1] IsInInspection - true
      (set `self.SavedTransform` (`SceneComponent.K2_GetComponentToWorld` (`self.picturealbum_low`)))
      (bind _asmurderer_script (cast `/Game/Blueprints/Character/MurdererScript` (`GameplayStatics.GetPlayerCharacter` 0)))
      (bind _inspectableobjectposition (`/Game/Blueprints/Character/MurdererScript.InspectableObjectPosition` _asmurderer_script))
      (`SceneComponent.K2_SetRelativeTransform` _inspectableobjectposition (`self.InspectionTransform`) false false)
      (`SceneComponent.K2_SetWorldTransform` (`self.picturealbum_low`) (`SceneComponent.K2_GetComponentToWorld` _inspectableobjectposition) false false)
      (`PrimitiveComponent.SetSimulatePhysics` (`self.picturealbum_low`) false)
      (`PrimitiveComponent.SetCollisionResponseToChannel` (`self.picturealbum_low`) "ECC_PhysicsBody" "ECR_Ignore")
      (set `self.IsInInspection` true))))

(event `/Game/Blueprints/Interfaces/IInteractable.IPositionReset`
  ;[1 1 1] IsInInspection - setFalse if linetrace misses
  (if (`self.IsInInspection`)
    (`PrimitiveComponent.SetSimulatePhysics` (`self.picturealbum_low`) true)
    (`SceneComponent.K2_SetWorldTransform` (`self.picturealbum_low`) (`self.SavedTransform`) false false)
    (set `self.IsInInspection` false)
    (else
      (`KismetSystemLibrary.PrintString` "Dont Reset"))))

(fn `PhotoAlbumGlowinessTimeCounter`
  (params (SavedDeltaSeconds :type "Float (double-precision)"))
  (bind _timephotoalbum (`self.TimePhotoAlbum`))
  (if (< _timephotoalbum (`self.MaxTimeGlowPhotoAlbum`))
    (set `self.TimePhotoAlbum` (+ SavedDeltaSeconds _timephotoalbum))
    (else
      (`/Engine/EditorBlueprintResources/StandardMacros.DoOnce` false
        (:`Completed`
          (set `self.GlowinessPhotoAlbum` true))))))

(fn `UserConstructionScript`)