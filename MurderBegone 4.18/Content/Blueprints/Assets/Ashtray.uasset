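; Inspectable ashtray prop that the MurdererScript player character can interact with.
; Tick runs a timer that starts an outline glow until interaction, creating a dynamic material instance every tick for Timelines to drive.
; Overlaps toggle input and MurdererScript's in-game notification, and C plays a one-shot voice-over through a gate.
; The inspection interface toggles the mesh between its saved transform with physics and the character's inspection position without physics.
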(event `Interact_1`
  ;[1 1 1] Interface - Interact
  (if (not (`self.IsAshTrayInteracted`))
    (set `self.IsAshTrayInteracted` true)))

(event `self.ReceiveTick`
  (params (DeltaSeconds :type "Float (single-precision)"))
  (bind _ashtray_unreal_ashtray_low (`self.ashtray_unreal_ashtray_low`))
  ;[1 0.3176 0] Event Tick - Animation Glow
  (`self.AshTrayGlowinessTimeCounter` DeltaSeconds)
  (if (and (== (`self.GlowinessAshTray`) true) (== (`self.IsAshTrayInteracted`) false))
    (bind _returnvalue (`PrimitiveComponent.CreateDynamicMaterialInstance` _ashtray_unreal_ashtray_low 0 null))
    (bind (_direction _newtrack_0) (`Timeline|Timeline_0`)
      (:`Update`
        (`MaterialInstanceDynamic.SetScalarParameterValue` _returnvalue "OutlineGlowPower (S)" _newtrack_0)))
    (else
      (bind _returnvalue_2 (`PrimitiveComponent.CreateDynamicMaterialInstance` _ashtray_unreal_ashtray_low 0 null))
      (bind (_direction_2 _newtrack_0_2) (`Timeline|Timeline_1`)
        (:`Update`
          (`MaterialInstanceDynamic.SetScalarParameterValue` _returnvalue_2 "OutlineGlowPower (S)" _newtrack_0_2))))))

(event `self.ReceiveActorEndOverlap`
  (params (OtherActor :type "Actor Object Reference"))
  ;[0 0 1] Enables Input when overlap
  (if (not (`PrimitiveComponent.IsOverlappingComponent` (`self.AshtrayCollision`) null))
    (`self.DisableInput` (`GameplayStatics.GetPlayerController` 0))))

(event `Key|C`
  (params (Key :type "Key Structure"))
  ;[0.3185 0 1] plays VoiceOver when button pressed
  (:`Pressed`
    (`/Engine/EditorBlueprintResources/StandardMacros.Gate` true :!label _label
      (:`Exit`
        (`/Engine/EditorBlueprintResources/StandardMacros.DoOnce` false
          (:`Completed`
            (`GameplayStatics.PlaySound2D` "/Game/Audio/VoiceOver/PlaceholderGate2/AshtrayInspectVO.AshtrayInspectVO")))))))

(event `self.ReceiveActorBeginOverlap`
  (params (OtherActor :type "Actor Object Reference"))
  ;[0 0 1] Enables Input when overlap
  (`KismetSystemLibrary.PrintText` "Ashtray")
  (`self.EnableInput` (`GameplayStatics.GetPlayerController` 0))
  (goto _label :!via `Open`))

(event `self.AshtrayCollision.OnComponentBeginOverlap`
  (params (OverlappedComponent :type "PrimitiveComponent Object Reference") (OtherActor :type "Actor Object Reference") (OtherComp :type "PrimitiveComponent Object Reference") (OtherBodyIndex :type Integer) (bFromSweep :type Boolean) (SweepResult :type "HitResult Structure (by ref)"))
  ;[1 1 1] execute creation for specific igame notifications
  (bind _outactors (`GameplayStatics.GetAllActorsOfClass` "/Game/Blueprints/Character/MurdererScript.MurdererScript_C"))
  (bind _output (`|GetArrayItem` _outactors))
  (set `/Game/Blueprints/Character/MurdererScript.ObjectNoteTags` (`self.ashtray_unreal_ashtray_low`) _output)
  (`/Game/Blueprints/Character/MurdererScript.CreateIngameNotification` _output))

(event `self.AshtrayCollision.OnComponentEndOverlap`
  (params (OverlappedComponent :type "PrimitiveComponent Object Reference") (OtherActor :type "Actor Object Reference") (OtherComp :type "PrimitiveComponent Object Reference") (OtherBodyIndex :type Integer))
  ;[1 1 1] execute creation for specific igame notifications
  (bind _outactors (`GameplayStatics.GetAllActorsOfClass` "/Game/Blueprints/Character/MurdererScript.MurdererScript_C"))
  (`/Game/Blueprints/Character/MurdererScript.DestroyIngameNotification` (`|GetArrayItem` _outactors)))

(event `/Game/Blueprints/Interfaces/IInteractable.IInspectionPosition`
  ;[1 1 1] Interface - IItemPosition
  (if (`self.IsInInspection`)
    ;;[1 1 1] IsInInspection - false
    (`PrimitiveComponent.SetSimulatePhysics` (`self.ashtray_unreal_ashtray_low`) true)
    (`SceneComponent.K2_SetWorldTransform` (`self.ashtray_unreal_ashtray_low`) (`self.SavedTransform`) false false)
    (set `self.IsInInspection` false)
    (else
      ;;[1 1 1] IsInInspection - true
      (set `self.SavedTransform` (`SceneComponent.K2_GetComponentToWorld` (`self.ashtray_unreal_ashtray_low`)))
      (bind _asmurderer_script (cast `/Game/Blueprints/Character/MurdererScript` (`GameplayStatics.GetPlayerCharacter` 0)))
      (bind _inspectableobjectposition (`/Game/Blueprints/Character/MurdererScript.InspectableObjectPosition` _asmurderer_script))
      (`SceneComponent.K2_SetRelativeTransform` _inspectableobjectposition (`self.InspectionTransform`) false false)
      (`SceneComponent.K2_SetWorldTransform` (`self.ashtray_unreal_ashtray_low`) (`SceneComponent.K2_GetComponentToWorld` _inspectableobjectposition) false false)
      (`PrimitiveComponent.SetSimulatePhysics` (`self.ashtray_unreal_ashtray_low`) false)
      (set `self.IsInInspection` true))))

(fn `AshTrayGlowinessTimeCounter`
  (params (SavedDeltaSeconds :type "Float (double-precision)"))
  (bind _timeashtray (`self.TimeAshTray`))
  (if (< _timeashtray (`self.MaxTimeGlowAshTray`))
    (set `self.TimeAshTray` (+ SavedDeltaSeconds _timeashtray))
    (else
      (`/Engine/EditorBlueprintResources/StandardMacros.DoOnce` false
        (:`Completed`
          (set `self.GlowinessAshTray` true))))))

(fn `UserConstructionScript`)