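; Interactive wine glass evidence prop that the player can inspect, wash or bleach, with voice-over lines.
; Interface events toggle it between its saved transform and the player's inspection point, switching physics, and drive notifications and glow.
; Tick animates the outline glow through dynamic materials and timelines; the timed glow helper is disconnected.
; Washing animates the material; both cleaning events raise MurdererScript's event counter and update its flags and inventory image.
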(event `self.ReceiveActorEndOverlap`
  (params (OtherActor :type "Actor Object Reference"))
  ;[0 0 1] enables input on overlap
  (if (not (`PrimitiveComponent.IsOverlappingComponent` (`self.UI Trigger`) null))
    (`self.DisableInput` (`GameplayStatics.GetPlayerController` 0))))

(event `self.ReceiveActorBeginOverlap`
  (params (OtherActor :type "Actor Object Reference"))
  ;[0 0 1] enables input on overlap
  (`KismetSystemLibrary.PrintText` "WineGlass")
  (`self.EnableInput` (`GameplayStatics.GetPlayerController` 0))
  (goto _label :!via `Open`))

(event `Key|C`
  (params (Key :type "Key Structure"))
  ;[0.3185 0 1] plays VoiceOver when pressed button
  (:`Pressed`
    (`/Engine/EditorBlueprintResources/StandardMacros.Gate` true :!label _label
      (:`Exit`
        (`/Engine/EditorBlueprintResources/StandardMacros.DoOnce` false
          (:`Completed`
            (`GameplayStatics.PlaySound2D` "/Game/Audio/VoiceOver/PlaceholderGate2/WineGlassInspectVO.WineGlassInspectVO")))))))

(event `self.ReceiveTick`
  (params (DeltaSeconds :type "Float (single-precision)"))
  ;[1 0.3176 0] Event Tick - Animation Glow
  (if (`self.GlowinessGlass`)
    (bind _returnvalue (`PrimitiveComponent.CreateDynamicMaterialInstance` (`self.Glass`) 0 null))
    (bind (_direction _newtrack_0) (`Timeline|Timeline_0`)
      (:`Update`
        (`MaterialInstanceDynamic.SetScalarParameterValue` _returnvalue "OutlineGlowPower (S)" _newtrack_0)
        (set `self.Hint_Glas` true)))
    (else
      (bind _returnvalue_2 (`PrimitiveComponent.CreateDynamicMaterialInstance` (`self.Glass`) 0 null))
      (bind (_direction_2 _newtrack_0_2) (`Timeline|Timeline_1`)
        (:`Update`
          (`MaterialInstanceDynamic.SetScalarParameterValue` _returnvalue_2 "OutlineGlowPower (S)" _newtrack_0_2)
          (set `self.Hint_Glas` false))))))

(event `BleachingWineGlass`
  ;[0.3185 0 1] Wine glass bleached event
  (`GameplayStatics.PlaySound2D` "/Game/Audio/VoiceOver/PlaceholderGate2/WineGlassInspectCleanVO.WineGlassInspectCleanVO")
  (bind _eventcount (`self.RaiseCounter`))
  (`KismetSystemLibrary.PrintString` (`KismetStringLibrary.Conv_IntToString` _eventcount))
  (bind _outactors (`GameplayStatics.GetAllActorsOfClass` "/Game/Blueprints/Character/MurdererScript.MurdererScript_C"))
  (bind _output (`|GetArrayItem` _outactors))
  (set `/Game/Blueprints/Character/MurdererScript.SlotItem` 6 _output)
  (set `/Game/Blueprints/Character/MurdererScript.isGlassBleached` true _output)
  (`/Game/Blueprints/Character/MurdererScript.IventoryImageChange` _output))

(event `WashingWineGlass`
  ;[0.3185 0 1] Washing Wine glass event
  (`PrimitiveComponent.SetSimulatePhysics` (`self.Glass`) false)
  (bind _returnvalue (`PrimitiveComponent.CreateDynamicMaterialInstance` (`self.Glass`) 0 null))
  (bind (_direction _newtrack_0) (`Timeline|Timeline_2`)
    (:`Update`
      (`MaterialInstanceDynamic.SetScalarParameterValue` _returnvalue "Time_In (S)" _newtrack_0))
    (:`Finished`
      (`GameplayStatics.PlaySound2D` "/Game/Audio/VoiceOver/PlaceholderGate2/WineGlassInspectSmudgeVO.WineGlassInspectSmudgeVO")
      (bind (_eventcount _wineglassbool _asmurdererscript) (`self.RaiseCounter`))
      (set `/Game/Blueprints/Character/MurdererScript.isGlassWashed` _wineglassbool _asmurdererscript)
      (`KismetSystemLibrary.PrintString` (`KismetStringLibrary.Conv_IntToString` _eventcount))
      (bind _outactors (`GameplayStatics.GetAllActorsOfClass` "/Game/Blueprints/Character/MurdererScript.MurdererScript_C"))
      (bind _output (`|GetArrayItem` _outactors))
      (set `/Game/Blueprints/Character/MurdererScript.SlotItem` 5 _output)
      (set `/Game/Blueprints/Character/MurdererScript.isGlassWashed` true _output)
      (`/Game/Blueprints/Character/MurdererScript.IventoryImageChange` _output)
      (`KismetSystemLibrary.Delay` 2.0)
      (`PrimitiveComponent.SetSimulatePhysics` (`self.Glass`) true)
      (`PrimitiveComponent.SetCollisionResponseToChannel` (`self.Glass`) "ECC_PhysicsBody" "ECR_Block"))))

(event `/Game/Blueprints/Interfaces/IInteractable.IInteract`
  ;[1 1 1] Interface-Interact
  (if (not (`self.IsGlassInteracted`))
    (set `self.IsGlassInteracted` true)))

(event `CreateNotes`
  ;[1 1 1] execute creation for specific igame notifications
  (bind _outactors (`GameplayStatics.GetAllActorsOfClass` "/Game/Blueprints/Character/MurdererScript.MurdererScript_C"))
  (bind _output (`|GetArrayItem` _outactors))
  (set `/Game/Blueprints/Character/MurdererScript.ObjectNoteTags` (`self.Glass`) _output)
  (`/Game/Blueprints/Character/MurdererScript.CreateIngameNotification` _output))

(event `/Game/Blueprints/Interfaces/IInteractable.IGlow`
  (params (GlowActive :type Boolean))
  ;[1 1 1] Interface-Interact
  (set `self.GlowinessGlass` GlowActive))

(event `DestroyNotes`
  ;[1 1 1] execute creation for specific igame notifications
  (bind _outactors (`GameplayStatics.GetAllActorsOfClass` "/Game/Blueprints/Character/MurdererScript.MurdererScript_C"))
  (`/Game/Blueprints/Character/MurdererScript.DestroyIngameNotification` (`|GetArrayItem` _outactors)))

(event `/Game/Blueprints/Interfaces/IInteractable.IInspectionPosition`
  (bind _glass (`self.Glass`))
  ;[1 1 1] Interface - IItemPosition
  (if (`self.IsInInspection`)
    ;;[1 1 1] IsInInspection - false
    (`PrimitiveComponent.SetSimulatePhysics` (`self.Glass`) true)
    (`SceneComponent.K2_SetWorldTransform` (`self.Glass`) (`self.SavedTransform`) false false)
    (`PrimitiveComponent.SetCollisionResponseToChannel` (`self.Glass`) "ECC_PhysicsBody" "ECR_Block")
    (set `self.IsInInspection` false)
    (else
      ;;[1 1 1] IsInInspection - true
      (set `self.SavedTransform` (`SceneComponent.K2_GetComponentToWorld` (`self.Glass`)))
      (bind _asmurderer_script (cast `/Game/Blueprints/Character/MurdererScript` (`GameplayStatics.GetPlayerCharacter` 0)))
      (bind _inspectableobjectposition (`/Game/Blueprints/Character/MurdererScript.InspectableObjectPosition` _asmurderer_script))
      (`SceneComponent.K2_SetRelativeTransform` _inspectableobjectposition (`self.InspectionTransform`) false false)
      (`SceneComponent.K2_SetWorldTransform` (`self.Glass`) (`SceneComponent.K2_GetComponentToWorld` _inspectableobjectposition) false false)
      (`PrimitiveComponent.SetSimulatePhysics` _glass false)
      (`PrimitiveComponent.SetCollisionResponseToChannel` _glass "ECC_PhysicsBody" "ECR_Ignore")
      (set `self.IsInInspection` true))))

(event `/Game/Blueprints/Interfaces/IInteractable.IPositionReset`
  ;[1 1 1] IsInInspection - setFalse if linetrace misses
  (if (`self.IsInInspection`)
    (`PrimitiveComponent.SetSimulatePhysics` (`self.Glass`) true)
    (`SceneComponent.K2_SetWorldTransform` (`self.Glass`) (`self.SavedTransform`) false false)
    (set `self.IsInInspection` false)
    (else
      (`KismetSystemLibrary.PrintString` "Dont Reset"))))

(fn `GlassGlowinessTimeCounter`
  (params (SavedDeltaSeconds :type "Float (double-precision)"))
  (bind _timeglass (`self.TimeGlass`))
  (if (< _timeglass (`self.MaxTimeGlowGlass`))
    (set `self.TimeGlass` (+ SavedDeltaSeconds _timeglass))
    (else
      (`/Engine/EditorBlueprintResources/StandardMacros.DoOnce` false
        (:`Completed`
          (set `self.GlowinessGlass` true))))))

(fn `RaiseCounter`
  (returns (EventCount :type Integer) (WineGlassBool :type Boolean) (AsMurdererScript :type "/Game/Blueprints/Character/MurdererScript Object Reference"))
  ;[1 1 1] raises counter for evaluation
  (bind _asmurderer_script (cast `/Game/Blueprints/Character/MurdererScript` (`GameplayStatics.GetPlayerCharacter` 0))
    (:`then`
      (bind _output_get (set `/Game/Blueprints/Character/MurdererScript.eventCounter` (+ (`/Game/Blueprints/Character/MurdererScript.eventCounter` _asmurderer_script) 1) _asmurderer_script))
      (return _output_get true _asmurderer_script))
    (:`CastFailed`
      (`KismetSystemLibrary.PrintString` "cast to failed"))))

(fn `UserConstructionScript`)