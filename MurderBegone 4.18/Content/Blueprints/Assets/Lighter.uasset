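; Lighter is an inspectable physics prop that implements interface events for inspection, interaction, glow and position reset.
; Inspection toggles: it saves the mesh transform and moves it to MurdererScript's InspectableObjectPosition with physics off and PhysicsBody collision ignored, then restores all three.
; Position reset, meant for linetrace misses, restores transform and physics but not the collision response.
; Interact latches a flag, and Glow only stores the value it receives.
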(event `/Game/Blueprints/Interfaces/IInteractable.IInspectionPosition`
  (bind _lighter_low (`self.lighter_low`))
  ;[1 1 1] Interface - IItemPosition
  (if (`self.IsInInspection`)
    ;;[1 1 1] IsInInspection - false
    (`PrimitiveComponent.SetSimulatePhysics` (`self.lighter_low`) true)
    (`SceneComponent.K2_SetWorldTransform` (`self.lighter_low`) (`self.SavedTransform`) false false)
    (`PrimitiveComponent.SetCollisionResponseToChannel` (`self.lighter_low`) "ECC_PhysicsBody" "ECR_Block")
    (set `self.IsInInspection` false)
    (else
      ;;[1 1 1] IsInInspection - true
      (set `self.SavedTransform` (`SceneComponent.K2_GetComponentToWorld` (`self.lighter_low`)))
      (bind _asmurderer_script (cast `/Game/Blueprints/Character/MurdererScript` (`GameplayStatics.GetPlayerCharacter` 0)))
      (bind _inspectableobjectposition (`/Game/Blueprints/Character/MurdererScript.InspectableObjectPosition` _asmurderer_script))
      (`SceneComponent.K2_SetRelativeTransform` _inspectableobjectposition (`self.InspectionTransform`) false false)
      (`SceneComponent.K2_SetWorldTransform` (`self.lighter_low`) (`SceneComponent.K2_GetComponentToWorld` _inspectableobjectposition) false false)
      (`PrimitiveComponent.SetSimulatePhysics` _lighter_low false)
      (`PrimitiveComponent.SetCollisionResponseToChannel` _lighter_low "ECC_PhysicsBody" "ECR_Ignore")
      (set `self.IsInInspection` true))))

(event `/Game/Blueprints/Interfaces/IInteractable.IInteract`
  ;[1 1 1] Interface-Interact
  (if (not (`self.IsLighterInteracted`))
    (set `self.IsLighterInteracted` true)))

(event `/Game/Blueprints/Interfaces/IInteractable.IPositionReset`
  ;[1 1 1] IsInInspection - setFalse if linetrace misses
  (if (`self.IsInInspection`)
    (`PrimitiveComponent.SetSimulatePhysics` (`self.lighter_low`) true)
    (`SceneComponent.K2_SetWorldTransform` (`self.lighter_low`) (`self.SavedTransform`) false false)
    (set `self.IsInInspection` false)
    (else
      (`KismetSystemLibrary.PrintString` "Dont Reset"))))

(event `/Game/Blueprints/Interfaces/IInteractable.IGlow`
  (params (GlowActive :type Boolean))
  ;[1 1 1] Interface-Interact
  (set `self.GlowinessLighter` GlowActive))

(fn `UserConstructionScript`)