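; Interactable toilet actor that lets the player toggle a flush sound with the E key.
; Overlapping the trigger component enables input and opens a Gate, whose FlipFlop alternately plays and stops the Spülen audio.
; Entering also has the first MurdererScript actor create an in-game notification tagged ToiletLow.
; Leaving disables input and destroys that notification, but never closes the Gate.
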(event `self.UI Ttigger.OnComponentBeginOverlap`
  (params (OverlappedComponent :type "PrimitiveComponent Object Reference") (OtherActor :type "Actor Object Reference") (OtherComp :type "PrimitiveComponent Object Reference") (OtherBodyIndex :type Integer) (bFromSweep :type Boolean) (SweepResult :type "HitResult Structure (by ref)"))
  (bind `_spülen` (`self.Spülen`))
  ;[0 0 1] enable input for gate, activates with button
  (`|ExecutionSequence`
    (:`then_0`
      (`self.EnableInput` (`GameplayStatics.GetPlayerController` 0))
      (goto _label :!via `Open`))
    (:`then_1`
      (`self.CreateNotes`))))

(event `Key|E`
  (params (Key :type "Key Structure"))
  (bind `_spülen` (`self.Spülen`))
  ;[0 0 1] enable input for gate, activates with button
  (:`Pressed`
    (`/Engine/EditorBlueprintResources/StandardMacros.Gate` true :!label _label
      (:`Exit`
        ;[0.3185 0 1] SFX: Toilet Flush
        (`/Engine/EditorBlueprintResources/StandardMacros.FlipFlop`
          (:`A`
            (`AudioComponent.Play` `_spülen` 0.0))
          (:`B`
            (`AudioComponent.Stop` `_spülen`)))))))

(event `self.UI Ttigger.OnComponentEndOverlap`
  (params (OverlappedComponent :type "PrimitiveComponent Object Reference") (OtherActor :type "Actor Object Reference") (OtherComp :type "PrimitiveComponent Object Reference") (OtherBodyIndex :type Integer))
  ;[0 0 1] enable input for gate, activates with button
  (`|ExecutionSequence`
    (:`then_0`
      (`self.DisableInput` (`GameplayStatics.GetPlayerController` 0)))
    (:`then_1`
      (`self.DestroyNotes`))))

(event `CreateNotes`
  ;[1 1 1] execute creation for specific igame notifications
  (bind _outactors (`GameplayStatics.GetAllActorsOfClass` "/Game/Blueprints/Character/MurdererScript.MurdererScript_C"))
  (bind _output (`|GetArrayItem` _outactors))
  (set `/Game/Blueprints/Character/MurdererScript.ObjectNoteTags` (`self.toilet_low`) _output)
  (`/Game/Blueprints/Character/MurdererScript.CreateIngameNotification` _output))

(event `DestroyNotes`
  ;[1 1 1] execute creation for specific igame notifications
  (bind _outactors (`GameplayStatics.GetAllActorsOfClass` "/Game/Blueprints/Character/MurdererScript.MurdererScript_C"))
  (`/Game/Blueprints/Character/MurdererScript.DestroyIngameNotification` (`|GetArrayItem` _outactors)))

(fn `UserConstructionScript`)