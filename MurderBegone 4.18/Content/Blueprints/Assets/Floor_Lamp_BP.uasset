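; Interactable floor lamp that toggles its light on and off through the IInteract interface event.
; A FlipFlop alternates the LampLight intensity and the mesh material's Emissive_Power parameter together, and each interaction prints a debug string.
; Box overlap begin and end set and clear NotificationTrigger on the MurdererScript actor for in-game notifications.
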(event `/Game/Blueprints/Interfaces/IInteractable.IInteract`
  (bind _lamp_light (`self.Lamp_Light`))
  ;[0.3185 0 1] Overlap_Trigger and Press "E"
  (`KismetSystemLibrary.PrintString` "Trace Light Switch" true true (struct :`R` 1.0 :`B` 0.84042 :`A` 1.0))
  (`/Engine/EditorBlueprintResources/StandardMacros.FlipFlop`
    (:`A`
      (`LightComponent.SetIntensity` _lamp_light 1000.0)
      (`MeshComponent.SetScalarParameterValueOnMaterials` (`self.floor_lamp`) "Emissive_Power" (`self.MaterialEmissivePowerOn`)))
    (:`B`
      (`LightComponent.SetIntensity` _lamp_light 0.0)
      (`MeshComponent.SetScalarParameterValueOnMaterials` (`self.floor_lamp`) "Emissive_Power" 0.0))))

(event `self.Box.OnComponentBeginOverlap`
  (params (OverlappedComponent :type "PrimitiveComponent Object Reference") (OtherActor :type "Actor Object Reference") (OtherComp :type "PrimitiveComponent Object Reference") (OtherBodyIndex :type Integer) (bFromSweep :type Boolean) (SweepResult :type "HitResult Structure (by ref)"))
  ;[1 1 1] execute creation for specific igame notifications
  (bind _asmurderer_script (cast `/Game/Blueprints/Character/MurdererScript` OtherActor))
  (if (not (`/Game/Blueprints/Character/MurdererScript.NotificationTrigger` _asmurderer_script))
    (set `/Game/Blueprints/Character/MurdererScript.NotificationTrigger` true _asmurderer_script)))

(event `self.Box.OnComponentEndOverlap`
  (params (OverlappedComponent :type "PrimitiveComponent Object Reference") (OtherActor :type "Actor Object Reference") (OtherComp :type "PrimitiveComponent Object Reference") (OtherBodyIndex :type Integer))
  ;[1 1 1] execute creation for specific igame notifications
  (bind _asmurderer_script (cast `/Game/Blueprints/Character/MurdererScript` OtherActor))
  (if (`/Game/Blueprints/Character/MurdererScript.NotificationTrigger` _asmurderer_script)
    (set `/Game/Blueprints/Character/MurdererScript.NotificationTrigger` false _asmurderer_script)))

(fn `UserConstructionScript`)