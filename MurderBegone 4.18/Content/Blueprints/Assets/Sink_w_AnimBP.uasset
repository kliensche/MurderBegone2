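; Interactive sink where pressing E inside the UI trigger runs a timed tap sequence of animation, sounds and water visibility.
; If the MurdererScript character holds a "knife"-tagged object, it also unhides the knife, plays a level sequence, and hides the knife afterwards.
; A capsule overlap with Knife_BP calls WashingKnife once, gated by IsTapOpen, which is set on first use and never reset.
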(event `self.UI Trigger.OnComponentBeginOverlap`
  (params (OverlappedComponent :type "PrimitiveComponent Object Reference") (OtherActor :type "Actor Object Reference") (OtherComp :type "PrimitiveComponent Object Reference") (OtherBodyIndex :type Integer) (bFromSweep :type Boolean) (SweepResult :type "HitResult Structure (by ref)"))
  ;[0 0 1] Overlap_Trigger and Press "E"
  (`self.EnableInput` (`GameplayStatics.GetPlayerController` 0))
  (goto _label :!via `Open`))

(event `Key|E`
  (params (Key :type "Key Structure"))
  ;[0 0 1] Overlap_Trigger and Press "E"
  (:`Pressed`
    (`/Engine/EditorBlueprintResources/StandardMacros.Gate` true :!label _label
      (:`Exit`
        ;[1 0 0] Tap_Animation_and_Sequence
        (`|ExecutionSequence`
          (:`then_0`
            ;;[1 1 1] unhide Knife
            (bind _asmurderer_script (cast `/Game/Blueprints/Character/MurdererScript` (`GameplayStatics.GetPlayerCharacter` 0))
              (:`then`
                (bind _pickupactor (`/Game/Blueprints/Character/MurdererScript.PickupActor` _asmurderer_script))
                (if (and (`self.ActorHasTag` _pickupactor "knife") (`/Game/Blueprints/Character/MurdererScript.Is_Holding_Object` _asmurderer_script))
                  ;;[1 1 1] Play Sequence only if knife is in hand
                  (`self.SetActorHiddenInGame` _pickupactor false)
                  (`MovieSceneSequencePlayer.Play` (`LevelSequenceActor.SequencePlayer` (`self.Sink_Sequence`))) ; Play Sequence
                  (`AudioComponent.Play` (`self.Tab`) 0.0)
                  (`SkeletalMeshComponent.PlayAnimation` (`self.Sink_new`) "/Game/VFX/Sink/Anim/Sink_new_TabClose_Anim.Sink_new_TabClose_Anim" false)
                  (`KismetSystemLibrary.Delay` 3.3333) ; delay to wait for Tab_Anim
                  (`SceneComponent.ToggleVisibility` (`self.Sink_water`) false)
                  (set `self.IsTapOpen` true)
                  (`AudioComponent.Play` (`self.Water_Start`) 0.0)
                  (`KismetSystemLibrary.Delay` 5.0) ; Time for Waterflow
                  (`AudioComponent.Play` (`self.Tab`) 0.0)
                  (`SkeletalMeshComponent.PlayAnimation` (`self.Sink_new`) "/Game/VFX/Sink/Anim/Sink_new_TabClose_Anim.Sink_new_TabClose_Anim" false)
                  (`AudioComponent.Play` (`self.Water_End`) 0.0)
                  (`KismetSystemLibrary.Delay` 3.3333)
                  (`SceneComponent.ToggleVisibility` (`self.Sink_water`) false)
                  (`AudioComponent.Stop` (`self.Water_Start`))
                  ;;[1 1 1] Hide Knife
                  (bind _asmurderer_script_2 (cast `/Game/Blueprints/Character/MurdererScript` (`GameplayStatics.GetPlayerCharacter` 0))
                    (:`then`
                      (`self.SetActorHiddenInGame` (`/Game/Blueprints/Character/MurdererScript.PickupActor` _asmurderer_script_2) true))
                    (:`CastFailed`
                      (`KismetSystemLibrary.PrintString` "cast to failed")))
                  (else
                    ;;[1 1 1] only opens sink and water + sound
                    (`AudioComponent.Play` (`self.Tab`) 0.0)
                    (`SkeletalMeshComponent.PlayAnimation` (`self.Sink_new`) "/Game/VFX/Sink/Anim/Sink_new_TabClose_Anim.Sink_new_TabClose_Anim" false)
                    (`KismetSystemLibrary.Delay` 3.3333) ; delay to wait for Tab_Anim
                    (`SceneComponent.ToggleVisibility` (`self.Sink_water`) false)
                    (set `self.IsTapOpen` true)
                    (`AudioComponent.Play` (`self.Water_Start`) 0.0)
                    (`KismetSystemLibrary.Delay` 5.0) ; Time for Waterflow
                    (`AudioComponent.Play` (`self.Tab`) 0.0)
                    (`SkeletalMeshComponent.PlayAnimation` (`self.Sink_new`) "/Game/VFX/Sink/Anim/Sink_new_TabClose_Anim.Sink_new_TabClose_Anim" false)
                    (`AudioComponent.Play` (`self.Water_End`) 0.0)
                    (`KismetSystemLibrary.Delay` 3.3333)
                    (`SceneComponent.ToggleVisibility` (`self.Sink_water`) false)
                    (`AudioComponent.Stop` (`self.Water_Start`)))))
              (:`CastFailed`
                (`KismetSystemLibrary.PrintString` "cast to failed")))))))))

(event `self.UI Trigger.OnComponentEndOverlap`
  (params (OverlappedComponent :type "PrimitiveComponent Object Reference") (OtherActor :type "Actor Object Reference") (OtherComp :type "PrimitiveComponent Object Reference") (OtherBodyIndex :type Integer))
  ;[0 0 1] Overlap_Trigger and Press "E"
  (`self.DisableInput` (`GameplayStatics.GetPlayerController` 0)))

(event `self.Capsule.OnComponentBeginOverlap`
  (params (OverlappedComponent :type "PrimitiveComponent Object Reference") (OtherActor :type "Actor Object Reference") (OtherComp :type "PrimitiveComponent Object Reference") (OtherBodyIndex :type Integer) (bFromSweep :type Boolean) (SweepResult :type "HitResult Structure (by ref)"))
  ;[0 0 1] wenn knife and water overlap -> event washing knife in knifeBP
  (if (`self.IsTapOpen`)
    (bind _asknife_bp (cast `/Game/Blueprints/Assets/Knife_BP` OtherActor)
      (:`then`
        (`/Engine/EditorBlueprintResources/StandardMacros.DoOnce` false
          (:`Completed`
            (`/Game/Blueprints/Assets/Knife_BP.WashingKnife` _asknife_bp)
            (`KismetSystemLibrary.PrintString` "cast to knife BP"))))
      (:`CastFailed`
        (`KismetSystemLibrary.PrintString` "cast to failed")))))

(fn `UserConstructionScript`)