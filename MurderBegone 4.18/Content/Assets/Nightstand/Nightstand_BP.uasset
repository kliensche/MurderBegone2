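; Nightstand Blueprint meant to open and close via a level sequence, though all its logic is currently disconnected and both trigger overlap events are empty.
; The unwired logic checks MurdererScript's pickup state to either pick up an object or enter a gate meant for trigger overlap.
; Past the gate, a FlipFlop plays NightstandAnim forward or in reverse, disabling input for a delay derived from IsPlaying cast to float.
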(event `self.Trigger.OnComponentBeginOverlap`
  (params (OverlappedComponent :type "PrimitiveComponent Object Reference") (OtherActor :type "Actor Object Reference") (OtherComp :type "PrimitiveComponent Object Reference") (OtherBodyIndex :type Integer) (bFromSweep :type Boolean) (SweepResult :type "HitResult Structure (by ref)"))
  ;[0.3185 0 1] Overlap_Trigger and Press "E"
)

(event `InputAction|PickUpInteract`
  (params (Key :type "Key Structure"))
  ;[0.3185 0 1] Overlap_Trigger and Press "E"
)

(event `self.Trigger.OnComponentEndOverlap`
  (params (OverlappedComponent :type "PrimitiveComponent Object Reference") (OtherActor :type "Actor Object Reference") (OtherComp :type "PrimitiveComponent Object Reference") (OtherBodyIndex :type Integer))
  ;[0.3185 0 1] Overlap_Trigger and Press "E"
)

(fn `UserConstructionScript`)