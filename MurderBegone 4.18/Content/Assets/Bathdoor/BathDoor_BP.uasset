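; Bathroom door Blueprint that lets the player open and close the door by pressing E inside a trigger.
; Trigger overlap enables input and opens a Gate, and leaving disables input.
; E passes the Gate into a FlipFlop that alternates playing the DoorSequence forward and in reverse.
; Input is disabled during a Delay derived from IsPlaying cast to float, about one second rather than the sequence's length.
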(event `self.Sequence_Trigger.OnComponentBeginOverlap`
  (params (OverlappedComponent :type "PrimitiveComponent Object Reference") (OtherActor :type "Actor Object Reference") (OtherComp :type "PrimitiveComponent Object Reference") (OtherBodyIndex :type Integer) (bFromSweep :type Boolean) (SweepResult :type "HitResult Structure (by ref)"))
  (bind _returnvalue (`GameplayStatics.GetPlayerController` 0))
  (bind _sequenceplayer (`LevelSequenceActor.SequencePlayer` (`self.Door_Sequence`)))
  (bind _sequenceplayer_2 (`LevelSequenceActor.SequencePlayer` (`self.Door_Sequence`)))
  (bind _returnvalue_2 (`MovieSceneSequencePlayer.IsPlaying` _sequenceplayer))
  ;[0.3185 0 1] Overlap_Trigger and Press "E"
  (`|ExecutionSequence`
    (:`then_0`
      (`self.EnableInput` (`GameplayStatics.GetPlayerController` 0))
      (goto _label :!via `Open`))))

(event `Key|E`
  (params (Key :type "Key Structure"))
  (bind _returnvalue (`GameplayStatics.GetPlayerController` 0))
  (bind _sequenceplayer (`LevelSequenceActor.SequencePlayer` (`self.Door_Sequence`)))
  (bind _sequenceplayer_2 (`LevelSequenceActor.SequencePlayer` (`self.Door_Sequence`)))
  (bind _returnvalue_2 (`MovieSceneSequencePlayer.IsPlaying` _sequenceplayer))
  ;[0.3185 0 1] Overlap_Trigger and Press "E"
  (:`Pressed`
    (`/Engine/EditorBlueprintResources/StandardMacros.Gate` true :!label _label
      (:`Exit`
        ;[1 0 0] Play sequence open and close
        (`/Engine/EditorBlueprintResources/StandardMacros.FlipFlop`
          (:`A`
            (`self.DisableInput` _returnvalue)
            (`MovieSceneSequencePlayer.SetPlaybackPosition` _sequenceplayer_2 0.0)
            (`MovieSceneSequencePlayer.Play` _sequenceplayer_2)
            (`KismetSystemLibrary.Delay` (`KismetMathLibrary.Conv_BoolToDouble` _returnvalue_2))
            (`self.EnableInput` _returnvalue))
          (:`B`
            (`self.DisableInput` _returnvalue)
            (`MovieSceneSequencePlayer.SetPlaybackPosition` _sequenceplayer (`MovieSceneSequencePlayer.GetPlaybackEnd` _sequenceplayer))
            (`MovieSceneSequencePlayer.PlayReverse` _sequenceplayer)
            (`KismetSystemLibrary.Delay` (`KismetMathLibrary.Conv_BoolToDouble` _returnvalue_2))
            (`self.EnableInput` _returnvalue)))))))

(event `self.Sequence_Trigger.OnComponentEndOverlap`
  (params (OverlappedComponent :type "PrimitiveComponent Object Reference") (OtherActor :type "Actor Object Reference") (OtherComp :type "PrimitiveComponent Object Reference") (OtherBodyIndex :type Integer))
  ;[0.3185 0 1] Overlap_Trigger and Press "E"
  (`|ExecutionSequence`
    (:`then_0`
      (`self.DisableInput` (`GameplayStatics.GetPlayerController` 0)))))

(fn `UserConstructionScript`)